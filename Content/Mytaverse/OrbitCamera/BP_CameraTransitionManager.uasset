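; Manager actor that handles named camera switching for the orbit camera system.
; On initialization it caches the orbit pawn, maps and initializes every BPI_CameraTarget actor by name, then selects the entry camera, which ResetToEntry also restores.
; SelectCamera exits the current target, waits its exit duration, then enters the new one, allowing re-selection only when that target permits it.
; Tick is forwarded to the current camera only.
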(event Custom|ResetToEntry
  (CallFunction|SelectCamera (Variables|Default|GetEntryCamera)))

(event Custom|SelectCamera
  (params (CameraName :type Name :default "None"))
  (bind (_returnvalue _bfindout) (CallFunction|FindCamerabyName CameraName))
  (if _bfindout
    (bind _returnvalue_2 (Class|BPICameraTarget|CanEnterfromSelf(Message) _returnvalue))
    (if _returnvalue_2
      (Class|BPICameraTarget|ExitCamera(Message) (Variables|Default|GetCurrentCamera) :!label _label) ; 需要一个过程
      (bind _output_get (Variables|Default|SetPreviousCamera (Variables|Default|GetCurrentCamera)))
      (bind _returnvalue_3 (Class|BPICameraTarget|GetExitDuration(Message) _output_get))
      (Utilities|FlowControl|Delay _returnvalue_3)
      (Class|BPICameraTarget|EnterCamera(Message) _returnvalue)
      (Variables|Default|SetCurrentCamera _returnvalue)
      (elif (!= (Variables|Default|GetCurrentCamera) _returnvalue)
        (goto _label)))))

(event Custom|Initialize
  (bind _returnvalue (Actor|GetActorOfClass "/Game/Mytaverse/OrbitCamera/BP_OrbitCameraPawn.BP_OrbitCameraPawn_C"))
  (Variables|Default|SetCameraPawn _returnvalue)
  (Utilities|Map|Clear (Variables|Default|GetCameraTargets))
  (bind _outactors (Actor|GetAllActorswithInterface "/Game/Mytaverse/OrbitCamera/BPI_CameraTarget.BPI_CameraTarget_C"))
  (for _array_element _outactors
    (bind _returnvalue_2 (Class|BPICameraTarget|GetName(Message) _array_element))
    (Utilities|Map|Add (Variables|Default|GetCameraTargets) _returnvalue_2 _array_element)
    (Class|BPICameraTarget|InitCamera(Message) _array_element self))
  (CallFunction|SelectCamera (Variables|Default|GetEntryCamera)))

(event EventTick
  (params (DeltaSeconds :type Float%20%28single-precision%29))
  (Class|BPICameraTarget|TickCamera(Message) (Variables|Default|GetCurrentCamera) DeltaSeconds))

(event EventBeginPlay
  (CallFunction|Initialize))

(fn ConstructionScript)

(fn FindCamerabyName
  (params (Key :type Name%20%28by%20ref%29))
  (bind _cameratargets (Variables|Default|GetCameraTargets))
  (bind (_value _returnvalue) (Utilities|Map|Find _cameratargets Key))
  (return _value (and (Utilities|IsValid _value) _returnvalue)))

(fn GetCurrentCamera
  (return (Variables|Default|GetCurrentCamera)))

(fn GetPreviousCamera
  (return (Variables|Default|GetPreviousCamera)))