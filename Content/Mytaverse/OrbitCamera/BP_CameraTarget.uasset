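; BP_CameraTarget is a placeable orbit camera position that stores its orbit settings and a reference to a camera transition manager.
; Its construction script positions OrbitCamera from view offsets and zoom distance, sets focal length, and derives the constraint base axis from actor yaw.
; An optional debug view scales meshes and drives material parameters to show zoom range and yaw/pitch limits.
; Enter and exit events only log the camera name; tick is empty.
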(event EventInitCamera
  (params (Manager :type BP%20Camera%20Transition%20Manager%20Object%20Reference))
  (Variables|Default|SetTransitionManager Manager))

(event EventEnterCamera
  (Development|PrintString (Utilities|String|Append "进入“" (Utilities|String|ToString(Name) (Variables|Default|GetCameraName)) "”相机机位") false))

(event EventTickCamera
  (params (DeltaTime :type Float%20%28double-precision%29)))

(event EventExitCamera
  (Development|PrintString (Utilities|String|Append "退出“" (Utilities|String|ToString(Name) (Variables|Default|GetCameraName)) "”相机机位") false))

(fn ConstructionScript
  (bind _returnvalue (Transformation|GetActorRotation))
  (bind _returnvalue_2 (Transformation|GetActorRotation))
  (bind _orbitcamerasettings (Variables|Default|GetOrbitCameraSettings))
  (bind _orbitcamerasettings_2 (Variables|Default|GetOrbitCameraSettings))
  (bind (_zoomdistance _focallength _maxpandistance _bpanscreenspace _horizontalviewoffset _verticalviewoffset) (Utilities|Struct|BreakFOrbitCameraSettings _orbitcamerasettings_2))
  (bind (_minpitchoffset _maxpitchoffset _minyawoffset _maxyawoffset _zoomdistance_2 _minzoomdistance _maxzoomdistance) (Utilities|Struct|BreakFOrbitCameraSettings _orbitcamerasettings))
  (Utilities|FlowControl|Sequence
    (:then_0
      (Transformation|SetRelativeLocation (Variables|Default|GetOrbitCamera) (Math|Vector|NegateVector (Class|KismetMathLibrary|CreateVectorfromYawPitch _horizontalviewoffset _verticalviewoffset _zoomdistance)) false false)
      (Variables|/Script/CinematicCamera.CineCameraComponent|SetCurrentFocalLength (Variables|Default|GetOrbitCamera) _focallength)
      (Transformation|SetActorRotation (Math|Rotator|MakeRotator 0.0 (.pitch _returnvalue) (.yaw _returnvalue)))
      (Utilities|Struct|SetmembersinFOrbitCameraSettings (Variables|Default|GetOrbitCameraSettings) (Math|Rotator|GetRotationXVector (Math|Rotator|MakeRotator 0.0 0.0 (.yaw (Transformation|GetActorRotation))))))
    (:then_1
      (if (Variables|Default|GetbDrawDebug)
        (Utilities|FlowControl|Sequence
          (:then_0
            (Rendering|SetVisibility (Variables|Default|GetDebugRoot) true true)
            (Transformation|SetWorldRotation (Variables|Default|GetDebugRoot) (Math|Conversions|RotationFromXVector (.ConstraintBaseAxis (Utilities|Struct|BreakFOrbitCameraSettings (Variables|Default|GetOrbitCameraSettings)))) false false)
            (Transformation|SetWorldRotation (Variables|Default|GetZoomLine) (Math|Rotator|MakeRotator 9e+01 (+ (.pitch _returnvalue_2) 1.8e+02) (.yaw _returnvalue_2)) false false))
          (:then_1
            (Transformation|SetRelativeScale3D (Variables|Default|GetDebugRoot) (Math|Conversions|ToVector(Float) _maxzoomdistance))
            (Transformation|SetWorldScale3D (Variables|Default|GetZoomLine) (Math|Conversions|ToVector(Float) _zoomdistance_2))
            (Rendering|Material|SetScalarParameterValueonMaterials (Variables|Default|GetOrbitYawAngle) "InnerRadius" (/ _minzoomdistance _maxzoomdistance))
            (Rendering|Material|SetScalarParameterValueonMaterials (Variables|Default|GetOrbitYawAngle) "MaxAngle" _maxyawoffset)
            (Rendering|Material|SetScalarParameterValueonMaterials (Variables|Default|GetOrbitYawAngle) "MinAngle" _minyawoffset)
            (Rendering|Material|SetScalarParameterValueonMaterials (Variables|Default|GetOrbitPitchAngle) "MaxAngle" _maxpitchoffset)
            (Rendering|Material|SetScalarParameterValueonMaterials (Variables|Default|GetOrbitPitchAngle) "MinAngle" _minpitchoffset)))
        (else
          (Rendering|SetVisibility (Variables|Default|GetDebugRoot) false true))))))

(fn GetCameraName
  (return (Variables|Default|GetCameraName)))

(fn GetTransitionManager
  (Variables|Default|GetTransitionManager
    (:then
      _)
    (:else
      (bind _returnvalue (Actor|GetActorOfClass "/Game/Mytaverse/OrbitCamera/BP_CameraTransitionManager.BP_CameraTransitionManager_C"))
      (Variables|Default|SetTransitionManager _returnvalue)))
  (return (Variables|Default|GetTransitionManager)))

(fn CanEnterfromSelf
  (return false))

(fn GetExitDuration
  (return 0.0))

(fn GetName
  (return (Variables|Default|GetCameraName)))