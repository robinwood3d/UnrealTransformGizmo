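; BP_OrbitCameraPawn_Test is a test pawn that drives orbit, pan and zoom camera controls from player input.
; Right and middle mouse buttons set held flags, which Tick reads to feed axis values into AddOrbitInput or AddPanInput, with orbit taking priority.
; Tick also passes an axis value to AddZoomInput every frame, regardless of buttons, after calling the parent Tick.
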(event EventTick
  (params (DeltaSeconds :type Float%20%28single-precision%29))
  (|CallParentFunction DeltaSeconds)
  (Utilities|FlowControl|Sequence
    (:then_0
      (if (Variables|Default|GetbRightMosuePressed)
        (CallFunction|AddOrbitInput (Math|Vector2D|MakeVector2D (Class|Actor|GetInputAxisKeyValue) (Class|Actor|GetInputAxisKeyValue)))
        (elif (Variables|Default|GetbMiddleMousePressed)
          (CallFunction|AddPanInput (Math|Vector2D|MakeVector2D (Class|Actor|GetInputAxisKeyValue) (Class|Actor|GetInputAxisKeyValue))))))
    (:then_1
      (CallFunction|AddZoomInput (Class|Actor|GetInputAxisKeyValue)))))

(event Input|MouseEvents|RightMouseButton
  (params (Key :type Key%20Structure :default "None"))
  (:Pressed
    (Variables|Default|SetbRightMosuePressed true))
  (:Released
    (Variables|Default|SetbRightMosuePressed false)))

(event Input|MouseEvents|MiddleMouseButton
  (params (Key :type Key%20Structure :default "None"))
  (:Pressed
    (Variables|Default|SetbMiddleMousePressed true))
  (:Released
    (Variables|Default|SetbMiddleMousePressed false)))

(fn ConstructionScript
  (|CallParentFunction))