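; A pointer touch component that turns raw touch input into tap, drag and pinch gesture events.
; Press, move and release events keep a map of finger positions and drive a None/Press/Drag/Pinch state machine that fires start and end callbacks.
; Tick compares current positions with the previous frame's to promote a press to a drag past a threshold and to report drag deltas or two-finger pan and zoom deltas.
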(event Custom|OnTouchPress
  (params (PointerIndex :type Byte%20%28by%20ref%29) (Position :type Vector%202D%20Structure))
  (bind _pointerpositions (Variables|Default|GetPointerPositions))
  (bind _pointerpositions_2 (Variables|Default|GetPointerPositions))
  (Utilities|Map|Add (Variables|Default|GetPointerPositions) PointerIndex Position)
  (Variables|Default|SetLastPointerPositions (Variables|Default|GetPointerPositions))
  (switch int (CallFunction|GetPointersNum)
    (:1
      (if (.ReturnValue (Utilities|Map|Find (Variables|Default|GetPointerPositions) 0))
        (switch Utilities|FlowControl|Switch|SwitchonEPointerTouchState (Variables|Default|GetTouchState)
          (:NewEnumerator7
            ;[1 1 1] 如果只有有一个触控点，且触控状态为None时，本次触控判定为进入Press状态
            (Variables|Default|SetTouchState "NewEnumerator12")
            (Default|CallOnTapDown (.Value (Utilities|Map|Find (Variables|Default|GetPointerPositions) 0)))))))
    (:2
      (if (and (.ReturnValue (Utilities|Map|Find _pointerpositions_2 0)) (.ReturnValue (Utilities|Map|Find _pointerpositions_2 1)))
        (switch Utilities|FlowControl|Switch|SwitchonEPointerTouchState (Variables|Default|GetTouchState)
          (:NewEnumerator7
            _)
          (:NewEnumerator12
            _)
          (:NewEnumerator4
            (Default|CallOnDragEnd (.Value (Utilities|Map|Find (Variables|Default|GetPointerPositions) 0))) ; 如果当前触控状态为Drag，则退出Drag状态
          ))
        ;[1 1 1] 当只有有两个触控点时，则进入Pinch状态
        (Variables|Default|SetTouchState "NewEnumerator10")
        (Default|CallOnPinchStart (CallFunction|Vector2dMultiplybyFloat (+ (.Value (Utilities|Map|Find _pointerpositions 0)) (.Value (Utilities|Map|Find _pointerpositions 1))) 0.5))))))

(event Custom|OnTouchMove
  (params (PointerIndex :type Byte) (Position :type Vector%202D%20Structure))
  (Utilities|Map|Add (Variables|Default|GetPointerPositions) PointerIndex Position))

(event Custom|OnTouchRelease
  (params (PointerIndex :type Byte) (Position :type Vector%202D%20Structure))
  (bind _pointerpositions (Variables|Default|GetPointerPositions))
  (bind _pointerpositions_2 (Variables|Default|GetPointerPositions))
  (Utilities|FlowControl|Sequence
    (:then_0
      (switch int (CallFunction|GetPointersNum)
        (:1
          (if (.ReturnValue (Utilities|Map|Find (Variables|Default|GetPointerPositions) 0))
            (switch Utilities|FlowControl|Switch|SwitchonEPointerTouchState (Variables|Default|GetTouchState)
              (:NewEnumerator12
                ;[1 1 1] 当只有一个触控点，该触控点松开，并且当前为Press状态时，触发TapUp
                (Variables|Default|SetTouchState "NewEnumerator7")
                (Default|CallOnTapUp (.Value (Utilities|Map|Find (Variables|Default|GetPointerPositions) 0))))
              (:NewEnumerator4
                ;[1 1 1] 当只有一个触控点，该触控点松开，并且当前为Drag状态时，触发DragEnd
                (Variables|Default|SetTouchState "NewEnumerator7")
                (Default|CallOnDragEnd (.Value (Utilities|Map|Find (Variables|Default|GetPointerPositions) 0)))))))
        (:2
          (if (and (.ReturnValue (Utilities|Map|Find _pointerpositions_2 0)) (.ReturnValue (Utilities|Map|Find _pointerpositions_2 1)))
            (switch Utilities|FlowControl|Switch|SwitchonEPointerTouchState (Variables|Default|GetTouchState)
              (:NewEnumerator10
                ;[1 1 1] 当存在两个触控点时，任一触控点松开，并且当前为Pinch状态时，触发PinchEnd
                (Variables|Default|SetTouchState "NewEnumerator7")
                (Default|CallOnPinchEnd (CallFunction|Vector2dMultiplybyFloat (+ (.Value (Utilities|Map|Find _pointerpositions 0)) (.Value (Utilities|Map|Find _pointerpositions 1))) 0.5))))))))
    (:then_1
      (Utilities|Map|Remove (Variables|Default|GetPointerPositions) PointerIndex)
      (Variables|Default|SetLastPointerPositions (Variables|Default|GetPointerPositions)))))

(event EventTick
  (params (DeltaSeconds :type Float%20%28single-precision%29))
  (bind _pointerpositions (Variables|Default|GetPointerPositions))
  (bind _pointerpositions_2 (Variables|Default|GetPointerPositions))
  (bind _value (Utilities|Map|Find _pointerpositions_2 0))
  (bind _value_2 (Utilities|Map|Find _pointerpositions_2 1))
  (Utilities|FlowControl|Sequence
    (:then_0
      (switch int (CallFunction|GetPointersNum)
        (:1
          (if (and (.ReturnValue (Utilities|Map|Find (Variables|Default|GetPointerPositions) 0)) (.ReturnValue (Utilities|Map|Find (Variables|Default|GetLastPointerPositions) 0)))
            (switch Utilities|FlowControl|Switch|SwitchonEPointerTouchState (Variables|Default|GetTouchState)
              (:NewEnumerator12
                ;[1 1 1] 当只有一个触控点，且触控状态为Press时，如果移动超过一定范围，则进入Drag状态
                (if (> (Math|Vector2D|Vector2DLength (- (.Value (Utilities|Map|Find (Variables|Default|GetPointerPositions) 0)) (.Value (Utilities|Map|Find (Variables|Default|GetLastPointerPositions) 0)))) (Variables|Default|GetDragThreshold))
                  (Variables|Default|SetTouchState "NewEnumerator4")
                  (Default|CallOnDragStart (.Value (Utilities|Map|Find (Variables|Default|GetPointerPositions) 0)))))
              (:NewEnumerator4
                ;[1 1 1] Drag状态更新
                (Default|CallOnDragMove (- (.Value (Utilities|Map|Find (Variables|Default|GetPointerPositions) 0)) (.Value (Utilities|Map|Find (Variables|Default|GetLastPointerPositions) 0))))))))
        (:2
          (if (Math|Boolean|ANDBoolean (.ReturnValue (Utilities|Map|Find _pointerpositions 0)) (.ReturnValue (Utilities|Map|Find _pointerpositions 1)) (.ReturnValue (Utilities|Map|Find (Variables|Default|GetLastPointerPositions) 0)) (.ReturnValue (Utilities|Map|Find (Variables|Default|GetLastPointerPositions) 1)))
            (switch Utilities|FlowControl|Switch|SwitchonEPointerTouchState (Variables|Default|GetTouchState)
              (:NewEnumerator10
                ;[1 1 1] 更新Pinch状态
                (Default|CallOnPinchMove (- (CallFunction|Vector2dMultiplybyFloat (+ _value _value_2) 0.5) (CallFunction|Vector2dMultiplybyFloat (+ (.Value (Utilities|Map|Find (Variables|Default|GetLastPointerPositions) 0)) (.Value (Utilities|Map|Find (Variables|Default|GetLastPointerPositions) 1))) 0.5)) (- (Math|Vector|Distance2D(Vector) _value _value_2) (Math|Vector|Distance2D(Vector) (.Value (Utilities|Map|Find (Variables|Default|GetLastPointerPositions) 0)) (.Value (Utilities|Map|Find (Variables|Default|GetLastPointerPositions) 1)))))))))))
    (:then_1
      (Variables|Default|SetLastPointerPositions (Variables|Default|GetPointerPositions)))))

(event Input|TouchEvents|InputTouch
  (params (Location :type Vector) (FingerIndex :type ETouchIndex%20Enum))
  (:Pressed
    (CallFunction|OnTouchPress FingerIndex (Math|Conversions|ToVector2D(Vector) Location)))
  (:Released
    (CallFunction|OnTouchRelease FingerIndex (Math|Conversions|ToVector2D(Vector) Location)))
  (:Moved
    (CallFunction|OnTouchMove FingerIndex (Math|Conversions|ToVector2D(Vector) Location))))

(fn GetPointersNum
  (bind _keys (Utilities|Map|Keys (Variables|Default|GetPointerPositions)))
  (return (Utilities|Array|Length _keys)))