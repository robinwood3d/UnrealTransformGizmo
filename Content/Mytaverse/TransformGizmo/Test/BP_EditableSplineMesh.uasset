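; Test actor for the transform gizmo: a spline mesh whose two ends are shaped by movable control point actors.
; On BeginPlay it spawns two BP_ControlPoint actors, at its origin and ahead along its forward vector, and binds to their OnTransformed events.
; Each transform is converted into spline mesh space to set that end's position, roll, cross-section scale (Y/Z) and tangent, with X scale controlling tangent length.
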(event Custom|Transform_ControlPointA
  (params (OutTransform :type Transform))
  (bind _splinemesh (Variables|Default|GetSplineMesh))
  (bind _splinemesh_2 (Variables|Default|GetSplineMesh))
  (bind _returnvalue (Transformation|GetWorldTransform _splinemesh_2))
  (bind _returnvalue_2 (Math|Transform|MakeRelativeTransform OutTransform _returnvalue))
  (bind (_location _rotation _scale) (Math|Transform|BreakTransform _returnvalue_2))
  (bind (_x _y _z) (Math|Vector|BreakVector _scale))
  (SplineMesh|SetStartPosition _splinemesh _location false)
  (Class|SplineMeshComponent|SetStartRoll _splinemesh (Math|Trig|DegreesToRadians (.Roll (Math|Rotator|BreakRotator _rotation))) false)
  (SplineMesh|SetStartScale _splinemesh (Math|Vector2D|MakeVector2D _y _z) false :!class /Script/Engine.SplineMeshComponent)
  (SplineMesh|SetStartTangent _splinemesh (* (Math|Vector|GetForwardVector _rotation) (* _x 1e+02)) true :!class /Script/Engine.SplineMeshComponent))

(event Custom|Transform_ControlPointB
  (params (OutTransform :type Transform))
  (bind _splinemesh (Variables|Default|GetSplineMesh))
  (bind _splinemesh_2 (Variables|Default|GetSplineMesh))
  (bind _returnvalue (Transformation|GetWorldTransform _splinemesh_2))
  (bind _returnvalue_2 (Math|Transform|MakeRelativeTransform OutTransform _returnvalue))
  (bind (_location _rotation _scale) (Math|Transform|BreakTransform _returnvalue_2))
  (bind (_x _y _z) (Math|Vector|BreakVector _scale))
  (SplineMesh|SetEndPosition _splinemesh _location false)
  (Class|SplineMeshComponent|SetEndRoll _splinemesh (Math|Trig|DegreesToRadians (.Roll (Math|Rotator|BreakRotator _rotation))) false)
  (SplineMesh|SetEndScale _splinemesh (Math|Vector2D|MakeVector2D _y _z) false :!class /Script/Engine.SplineMeshComponent)
  (SplineMesh|SetEndTangent _splinemesh (* (Math|Vector|GetForwardVector _rotation) (* _x 1e+02)) true :!class /Script/Engine.SplineMeshComponent))

(event EventBeginPlay
  (bind _returnvalue (Transformation|GetActorLocation))
  (Utilities|FlowControl|Sequence
    (:then_0
      (bind _returnvalue_2 (Game|SpawnActorfromClass "/Game/Mytaverse/TransformGizmo/Test/BP_ControlPoint.BP_ControlPoint_C" (Math|Transform|MakeTransform _returnvalue) "AlwaysSpawn" 0 0))
      (bind _output_get (Variables|Default|SetControlPointA _returnvalue_2))
      (EventDispatchers|BindEventtoOnTransformed _output_get (delegate Custom|Transform_ControlPointA)))
    (:then_1
      (bind _returnvalue_3 (Game|SpawnActorfromClass "/Game/Mytaverse/TransformGizmo/Test/BP_ControlPoint.BP_ControlPoint_C" (Math|Transform|MakeTransform (+ _returnvalue (* (Transformation|GetActorForwardVector) 5e+02))) "AlwaysSpawn" 0 0))
      (bind _output_get_2 (Variables|Default|SetControlPointB _returnvalue_3))
      (EventDispatchers|BindEventtoOnTransformed _output_get_2 (delegate Custom|Transform_ControlPointB)))
    (:then_2
      (CallFunction|TransformControlPointA (Transformation|GetActorTransform (Variables|Default|GetControlPointA)))
      (CallFunction|TransformControlPointB (Transformation|GetActorTransform (Variables|Default|GetControlPointB))))))

(fn ConstructionScript)