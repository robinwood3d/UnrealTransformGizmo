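; Clickable control point actor in the TransformGizmo test folder that can be moved with BP_TransformGizmo.
; Pointer down activates the first gizmo found in the level at the point's transform, passing a transform event.
; OnHandleTransform applies the incoming transform to the actor and broadcasts OnTransformed.
; Tick scales the absolute-scale Sphere by camera view depth, within clamps, to hold a constant on-screen size.
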(event EventBeginPlay
  (Transformation|SetAbsolute (Variables|Default|GetSphere) false false true))

(event EventTick
  (params (DeltaSeconds :type Float%20%28single-precision%29))
  (bind _returnvalue (Game|GetPlayerCameraManager 0))
  (Transformation|SetWorldScale3D (Variables|Default|GetSphere) (Math|Conversions|ToVector(Float) (Math|Float|Clamp(Float) (* (Math|Vector|DotProduct (- (Transformation|GetActorLocation) (Camera|GetCameraLocation _returnvalue)) (Math|Vector|GetForwardVector (Camera|GetCameraRotation _returnvalue))) 0.0005) 0.0001 1e+03))))

(fn ConstructionScript)

(fn OnHandleTransform
  (params (Transform :type Transform))
  (Transformation|SetActorTransform Transform)
  (Default|CallOnTransformed (Transformation|GetActorTransform)))

(fn GetHitPriority
  (params (Pointer :type BP%20Pointer%20Interaction%20Component%20Object%20Reference) (Component :type Primitive%20Component%20Object%20Reference))
  (return 0))

(fn IgnoreHitTest
  (params (Pointer :type BP%20Pointer%20Interaction%20Component%20Object%20Reference) (Component :type Primitive%20Component%20Object%20Reference))
  (return false))

(fn OnPointerDown
  (params (Pointer :type BP%20Pointer%20Interaction%20Component%20Object%20Reference) (Component :type Primitive%20Component%20Object%20Reference))
  (bind _returnvalue (Actor|GetActorOfClass "/Game/Mytaverse/TransformGizmo/BP_TransformGizmo.BP_TransformGizmo_C"))
  (Default|ActivateGizmo _returnvalue (Transformation|GetActorTransform) (EventDispatchers|CreateEvent :!event OnHandleTransform))
  (return false))