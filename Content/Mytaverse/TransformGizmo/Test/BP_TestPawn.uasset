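; BP_TestPawn is a test pawn for the TransformGizmo feature that drives mouse-based pointer interaction.
; On BeginPlay it shows the cursor and configures BPPointerInteractionComponent for very long-range, multi-hit traces on complex collision of WorldDynamic objects.
; Left mouse press and release are forwarded to the component as pointer press and release, with look input ignored while the button is held.
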(event EventBeginPlay
  (Variables|/Script/Engine.PlayerController|SetbShowMouseCursor (Game|GetPlayerController 0) true)
  (Default|SetupInteraction (Variables|Default|GetBP_PointerInteractionComponent) (Utilities|Struct|MakeFPointerInteractionSettings "NewEnumerator9" 1e+08 true 0.0 (Utilities|Array|MakeArray "ObjectTypeQuery2") true 0) true))

(event Input|MouseEvents|LeftMouseButton
  (params (Key :type Key%20Structure))
  (bind _returnvalue (Game|GetPlayerController 0))
  (bind _bp_pointerinteractioncomponent (Variables|Default|GetBP_PointerInteractionComponent))
  (:Pressed
    (Default|PressPointer _bp_pointerinteractioncomponent)
    (Input|SetIgnoreLookInput _returnvalue true))
  (:Released
    (Default|ReleasePointer _bp_pointerinteractioncomponent)
    (Input|SetIgnoreLookInput _returnvalue false)))

(fn ConstructionScript)