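; Actor component for PointVR Toolkit that drives hover, click and drag interaction from line, predicted-projectile or cursor traces.
; Each tick it traces and diffs the hit against the hovered actor and component, messaging enter, move, leave and hover changes through BPI_ToolkitTraceInteractive.
; Click events forward to the hovered actor, whose drag-start reply enables per-frame drag updates.
; Hover can be locked or set manually, and deactivation clears interaction state.
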(event Custom|TraceHoverInteraction
  (params (TraceHit :type Hit%20Result%20Structure%20%28by%20ref%29))
  (bind (_bblockinghit _binitialoverlap _time _distance _location _impactpoint _normal _impactnormal _physmat _hitactor _hitcomponent) (Collision|BreakHitResult TraceHit))
  ;[1 0 0] 处理每帧的悬浮交互        Inspired By mitchemmc's Excellent Blueprint (https://github.com/mitchemmc/VRContentExamples)                强调一下，在交互的过程中如果你想摧毁某个交互中的对象，请不要直接Destroy，而是先隐形并关闭碰撞，过一会在删掉
  ;;[1 1 0] 和之前碰到的是同一个Actor吗
  (if (== (Variables|TraceData|GetHoveredActor) _hitactor)
    (Class|BPIToolkitTraceInteractive|OnTraceMove(Message) (Variables|TraceData|GetHoveredActor) self TraceHit)
    ;;[1 1 0] 和之前碰到的是同一个Component吗
    (if (not (== (Variables|TraceData|GetHoveredComponent) _hitcomponent))
      (Class|BPIToolkitTraceInteractive|OnComponentUnhovered(Message) (Variables|TraceData|GetHoveredActor) self TraceHit (Variables|TraceData|GetHoveredComponent))
      (Variables|TraceData|SetHoveredComponent 0)
      (Class|BPIToolkitTraceInteractive|OnComponentHovered(Message) (Variables|TraceData|GetHoveredActor) self TraceHit _hitcomponent)
      (Variables|TraceData|SetHoveredComponent _hitcomponent))
    (else
      (Class|BPIToolkitTraceInteractive|OnTraceLeave(Message) (Variables|TraceData|GetHoveredActor) self TraceHit)
      (Class|BPIToolkitTraceInteractive|OnComponentUnhovered(Message) (Variables|TraceData|GetHoveredActor) self TraceHit (Variables|TraceData|GetHoveredComponent))
      (Variables|TraceData|SetHoveredActor 0)
      (Variables|TraceData|SetHoveredComponent 0)
      ;;[1 1 0] 检查是否实现了接口
      (if (Utilities|DoesObjectImplementInterface _hitactor "/Game/PointVRToolkit/Blueprints/Interfaces/BPI_ToolkitTraceInteractive.BPI_ToolkitTraceInteractive_C")
        (Class|BPIToolkitTraceInteractive|OnTraceEnter(Message) _hitactor self TraceHit)
        (Class|BPIToolkitTraceInteractive|OnComponentHovered(Message) _hitactor self TraceHit _hitcomponent)
        (Variables|TraceData|SetHoveredActor _hitactor)
        (Variables|TraceData|SetHoveredComponent _hitcomponent)))))

(event Custom|ClickPressed
  ;[1 1 0] 捡取
  (Class|BPIToolkitTraceInteractive|OnClickPressed(Message) (Variables|TraceData|GetHoveredActor) self (Variables|TraceData|GetTraceHit))
  ;[1 1 0] 拖拽
  (bind _returnvalue (Class|BPIToolkitTraceInteractive|OnDragStarted(Message) (Variables|TraceData|GetHoveredActor) self (Variables|TraceData|GetTraceHit)))
  (Variables|Default|SetbIsDragging _returnvalue))

(event Custom|DeactivateInteraction
  ;[1 1 0] 交互逻辑的开启与关闭
  (Variables|Default|SetbIsInteractionActivated false)
  (CallFunction|ClickReleased)
  (Class|BPIToolkitTraceInteractive|OnComponentUnhovered(Message) (Variables|TraceData|GetHoveredActor) self (Variables|TraceData|GetTraceHit) (Variables|TraceData|GetHoveredComponent))
  (Variables|TraceData|SetHoveredComponent 0)
  (Class|BPIToolkitTraceInteractive|OnTraceLeave(Message) (Variables|TraceData|GetHoveredActor) self (Variables|TraceData|GetTraceHit))
  (Variables|TraceData|SetHoveredActor 0)
  (Variables|TraceData|SetTraceHit ""))

(event Custom|ActivateInteraction
  ;[1 1 0] 交互逻辑的开启与关闭
  (Variables|Default|SetbIsInteractionActivated true))

(event Custom|ClickReleased
  ;[1 1 0] 捡取
  (Class|BPIToolkitTraceInteractive|OnClickReleased(Message) (Variables|TraceData|GetHoveredActor) self (Variables|TraceData|GetTraceHit))
  ;[1 1 0] 拖拽
  (Class|BPIToolkitTraceInteractive|OnDragEnded(Message) (Variables|TraceData|GetHoveredActor) self (Variables|TraceData|GetTraceHit))
  (Variables|Default|SetbIsDragging false))

(event Custom|SetupInteractor
  (params (TraceMode :type ETraceMode%20Enum :default "NewEnumerator0") (TraceObjectType :type Array%20of%20EObjectTypeQuery%20Enums :default "ObjectTypeQuery1") (LineDistance :type Float%20%28single-precision%29) (ProjectileVelocity :type Float%20%28single-precision%29) (DirectionComponent :type Scene%20Component%20Object%20Reference))
  ;[1 1 0] 交互组件的设置，该部分直接改变交互形式
  (if (Variables|Default|GetbIsInteractionActivated)
    (CallFunction|DeactivateInteraction))
  (Variables|TraceSettings|SetTraceMode TraceMode)
  (Variables|TraceSettings|SetTraceObjectType TraceObjectType)
  (Variables|TraceSettings|SetLineDistance LineDistance)
  (Variables|TraceSettings|SetProjectileVelocity ProjectileVelocity)
  (Variables|TraceSettings|SetTraceDirectionComponent DirectionComponent)
  (CallFunction|ActivateInteraction))

(event Custom|UnlockHovered
  ;[1 1 0] 交互对象的锁定与解锁，一般用于防止在和对象交互时被另一个对象打断
  (Variables|Default|SetbLockOnHovered false))

(event Custom|LockHovered
  ;[1 1 0] 交互对象的锁定与解锁，一般用于防止在和对象交互时被另一个对象打断
  (Variables|Default|SetbLockOnHovered true))

(event Custom|SetCustomHovered
  (params (CustomActor :type Actor%20Object%20Reference) (CustomComponent :type Primitive%20Component%20Object%20Reference) (Lock :type Boolean))
  ;[1 1 0] 手动设置交互对象
  (Variables|TraceData|SetHoveredActor CustomActor)
  (Variables|TraceData|SetHoveredComponent CustomComponent)
  (if Lock
    (CallFunction|LockHovered)
    (else
      (CallFunction|UnlockHovered))))

(event EventTick
  (params (DeltaSeconds :type Float%20%28single-precision%29))
  ;[1 0 0] Trace交互的核心逻辑
  (if (Variables|Default|GetbIsInteractionActivated)
    (Utilities|FlowControl|Sequence
      (:then_0
        (if (not (Variables|Default|GetbLockOnHovered))
          (bind _tracehit (CallFunction|EventTrace (Variables|TraceSettings|GetTraceMode) (Variables|TraceSettings|GetTraceObjectType) (Variables|TraceSettings|GetTraceDirectionComponent)))
          (bind _output_get (Variables|TraceData|SetTraceHit _tracehit))
          (CallFunction|TraceHoverInteraction _output_get)))
      (:then_1
        ;;[1 1 0] 逐帧拖拽
        (if (Variables|Default|GetbIsDragging)
          (Class|BPIToolkitTraceInteractive|OnDragMoved(Message) (Variables|TraceData|GetHoveredActor) self (Variables|TraceData|GetTraceHit)))))))

(fn EventTrace
  (params (TraceMode :type ETraceMode%20Enum :default "NewEnumerator0") (TraceChannel :type Array%20of%20EObjectTypeQuery%20Enums :default "ObjectTypeQuery1") (DirectionComponent :type Scene%20Component%20Object%20Reference))
  (bind _returnvalue (Transformation|GetWorldLocation DirectionComponent))
  (switch Utilities|FlowControl|Switch|SwitchonETraceMode TraceMode
    (:NewEnumerator0
      (bind _outhit (Collision|LineTraceForObjects _returnvalue (+ _returnvalue (* (Math|Vector|GetForwardVector DirectionComponent) (Variables|TraceSettings|GetLineDistance))) TraceChannel false 0 "None"))
      (return _outhit))
    (:NewEnumerator2
      (bind (_outhit_2 _outpathpositions) (Class|GameplayStatics|BlueprintPredictProjectilePathbyObjectType (Transformation|GetWorldLocation DirectionComponent) (* (Math|Vector|GetForwardVector DirectionComponent) (Variables|TraceSettings|GetProjectileVelocity)) true 0.0 TraceChannel false 0 "None"))
      (Variables|TraceData|SetProjectPath _outpathpositions)
      (return _outhit_2))
    (:NewEnumerator1
      (return (.HitResult (Class|PlayerController|GetHitResultUnderCursorforObjects (Game|GetPlayerController 0) TraceChannel true))))))

(fn GetTraceHit
  (return (Variables|TraceData|GetTraceHit)))

(fn GetHoveredResult
  (return (Variables|TraceData|GetHoveredActor) (Variables|TraceData|GetHoveredComponent)))