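; Runtime transform gizmo in PointVRToolkit that rotates and scales a target component, with mode switching toggling handle visibility and collision, defaulting to Scale.
; A handle map supplies mode, space and axis to hover highlighting and drag callbacks.
; Drags project mouse movement onto screen-space axes, while the trackball uses arcball rotation.
; The gizmo scales with camera distance; translation handles switch and highlight but have no drag logic.
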(event EventBeginPlay
  (CallFunction|SwitchTransformMode "NewEnumerator2"))

(event EventTick
  (params (DeltaSeconds :type Float%20%28single-precision%29))
  (CallFunction|UpdateGizmoScale))

(fn ConstructionScript
  (CallFunction|SwitchTransformMode "NewEnumerator2")
  (CallFunction|InitialTransformHandleIdentity))

(fn SwitchTransformMode
  (params (TransformMode :type ETransformMode%20Enum :default "NewEnumerator0"))
  (switch Utilities|FlowControl|Switch|SwitchonETransformMode TransformMode
    (:NewEnumerator0
      (Translation|SetActiveTranslationGizmo true)
      (Rotation|SetActiveRotationGizmo false)
      (Scale|SetActiveScaleGizmo false))
    (:NewEnumerator1
      (Translation|SetActiveTranslationGizmo false)
      (Rotation|SetActiveRotationGizmo true)
      (Scale|SetActiveScaleGizmo false))
    (:NewEnumerator2
      (Translation|SetActiveTranslationGizmo false)
      (Rotation|SetActiveRotationGizmo false)
      (Scale|SetActiveScaleGizmo true))))

(fn SetActiveRotationGizmo
  (params (NewActive :type Boolean))
  (bind _trackballhandle (Variables|TransformHandle|GetTrackBallHandle))
  (Rendering|SetVisibility (Variables|Default|GetRotationGizmoRoot) NewActive true)
  (if NewActive
    (Collision|SetCollisionEnabled _trackballhandle "QueryOnly")
    (else
      (Collision|SetCollisionEnabled _trackballhandle "NoCollision"))))

(fn SetActiveScaleGizmo
  (params (NewActive :type Boolean))
  (bind _uniformscalehandle (Variables|TransformHandle|GetUniformScaleHandle))
  (Rendering|SetVisibility (Variables|Default|GetScaleGizmoRoot) NewActive true)
  (if NewActive
    (Collision|SetCollisionEnabled _uniformscalehandle "QueryOnly")
    (else
      (Collision|SetCollisionEnabled _uniformscalehandle "NoCollision"))))

(fn SetActiveTranslationGizmo
  (params (NewActive :type Boolean))
  (bind _freetranslationhandle (Variables|TransformHandle|GetFreeTranslationHandle))
  (Rendering|SetVisibility (Variables|Default|GetTranslationGizmoRoot) NewActive true)
  (if NewActive
    (Collision|SetCollisionEnabled _freetranslationhandle "QueryOnly")
    (else
      (Collision|SetCollisionEnabled _freetranslationhandle "NoCollision"))))

(fn UpdateGizmoScale
  (bind _returnvalue (Game|GetPlayerCameraManager 0))
  (bind _returnvalue_2 (Transformation|GetActorLocation))
  (bind _gizmoscale (Variables|GizmoSettings|GetGizmoScale))
  (bind _returnvalue_3 (Camera|GetCameraLocation _returnvalue))
  (bind _returnvalue_4 (Math|Vector|Distance(Vector) _returnvalue_3 _returnvalue_2))
  (bind _returnvalue_5 (/ _returnvalue_4 5e+02))
  (bind _returnvalue_6 (* _returnvalue_5 _gizmoscale))
  (Transformation|SetActorScale3D (Math|Conversions|ToVector(Float) _returnvalue_6))
  (Variables|GizmoSettings|SetTrackballRadius (* _returnvalue_6 5e+01)))

(fn InitialTransformHandleIdentity
  (bind _transformhandleidentity (Variables|GizmoIdentity|GetTransformHandleIdentity))
  (Utilities|Map|Clear _transformhandleidentity) ; 拖动Actor的时候构造脚本会持续运行，填充大量垃圾数据，不清楚运行时会不会自动清空这些无用数据，我这里保险起见先清空了
  ;[1 1 0] Translation移动
  (Utilities|Map|Add _transformhandleidentity (Variables|TransformHandle|GetFreeTranslationHandle) (Utilities|Struct|MakeSTransformHandleIdentity "NewEnumerator0" "NewEnumerator1" "NewEnumerator8"))
  (Utilities|Map|Add _transformhandleidentity (Variables|TransformHandle|GetTranslationHandleXAxis) (Utilities|Struct|MakeSTransformHandleIdentity "NewEnumerator0" "NewEnumerator1" "NewEnumerator0"))
  (Utilities|Map|Add _transformhandleidentity (Variables|TransformHandle|GetTranslationHandleYAxis) (Utilities|Struct|MakeSTransformHandleIdentity "NewEnumerator0" "NewEnumerator1" "NewEnumerator1"))
  (Utilities|Map|Add _transformhandleidentity (Variables|TransformHandle|GetTranslationHandleZAxis) (Utilities|Struct|MakeSTransformHandleIdentity "NewEnumerator0" "NewEnumerator1" "NewEnumerator2"))
  (Utilities|Map|Add _transformhandleidentity (Variables|TransformHandle|GetTranslationHandleYZAxis) (Utilities|Struct|MakeSTransformHandleIdentity "NewEnumerator0" "NewEnumerator1" "NewEnumerator11"))
  (Utilities|Map|Add _transformhandleidentity (Variables|TransformHandle|GetTranslationHandleXZAxis) (Utilities|Struct|MakeSTransformHandleIdentity "NewEnumerator0" "NewEnumerator1" "NewEnumerator10"))
  (Utilities|Map|Add _transformhandleidentity (Variables|TransformHandle|GetTranslationHandleXYAxis) (Utilities|Struct|MakeSTransformHandleIdentity "NewEnumerator0" "NewEnumerator1" "NewEnumerator9"))
  ;[1 1 0] Rotation旋转，目前我旋转只有Local坐标系下执行
  (Utilities|Map|Add _transformhandleidentity (Variables|TransformHandle|GetTrackBallHandle) (Utilities|Struct|MakeSTransformHandleIdentity "NewEnumerator1" "NewEnumerator1" "NewEnumerator8"))
  (Utilities|Map|Add _transformhandleidentity (Variables|TransformHandle|GetRotationHandleXAxis) (Utilities|Struct|MakeSTransformHandleIdentity "NewEnumerator1" "NewEnumerator0" "NewEnumerator0"))
  (Utilities|Map|Add _transformhandleidentity (Variables|TransformHandle|GetRotationHandleYAxis) (Utilities|Struct|MakeSTransformHandleIdentity "NewEnumerator1" "NewEnumerator0" "NewEnumerator1"))
  (Utilities|Map|Add _transformhandleidentity (Variables|TransformHandle|GetRotationHandleZAxis) (Utilities|Struct|MakeSTransformHandleIdentity "NewEnumerator1" "NewEnumerator0" "NewEnumerator2"))
  ;[1 1 0] Scale缩放，缩放一般也只有在Local坐标系下执行
  (Utilities|Map|Add _transformhandleidentity (Variables|TransformHandle|GetUniformScaleHandle) (Utilities|Struct|MakeSTransformHandleIdentity "NewEnumerator2" "NewEnumerator0" "NewEnumerator8"))
  (Utilities|Map|Add _transformhandleidentity (Variables|TransformHandle|GetScaleHandleXAxis) (Utilities|Struct|MakeSTransformHandleIdentity "NewEnumerator2" "NewEnumerator0" "NewEnumerator0"))
  (Utilities|Map|Add _transformhandleidentity (Variables|TransformHandle|GetScaleHandleYAxis) (Utilities|Struct|MakeSTransformHandleIdentity "NewEnumerator2" "NewEnumerator0" "NewEnumerator1"))
  (Utilities|Map|Add _transformhandleidentity (Variables|TransformHandle|GetScaleHandleZAxis) (Utilities|Struct|MakeSTransformHandleIdentity "NewEnumerator2" "NewEnumerator0" "NewEnumerator2"))
  (Utilities|Map|Add _transformhandleidentity (Variables|TransformHandle|GetScaleHandleYZAxis) (Utilities|Struct|MakeSTransformHandleIdentity "NewEnumerator2" "NewEnumerator0" "NewEnumerator11"))
  (Utilities|Map|Add _transformhandleidentity (Variables|TransformHandle|GetScaleHandleXZAxis) (Utilities|Struct|MakeSTransformHandleIdentity "NewEnumerator2" "NewEnumerator0" "NewEnumerator10"))
  (Utilities|Map|Add _transformhandleidentity (Variables|TransformHandle|GetScaleHandleXYAxis) (Utilities|Struct|MakeSTransformHandleIdentity "NewEnumerator2" "NewEnumerator0" "NewEnumerator9")))

(fn SetTransformTarget
  (params (TransformTarget :type Scene%20Component%20Object%20Reference))
  (Variables|TransformTarget|SetTransformTargetRoot TransformTarget))

(fn OnClickPressed
  (params (Interactor :type BPC%20Toolkit%20Trace%20Interactor%20Object%20Reference) (TraceHit :type Hit%20Result%20Structure%20%28by%20ref%29))
  (return false))

(fn OnClickReleased
  (params (Interactor :type BPC%20Toolkit%20Trace%20Interactor%20Object%20Reference) (TraceHit :type Hit%20Result%20Structure%20%28by%20ref%29))
  (return false))

(fn OnComponentHovered
  (params (Interactor :type BPC%20Toolkit%20Trace%20Interactor%20Object%20Reference) (TraceHit :type Hit%20Result%20Structure%20%28by%20ref%29) (CurrentComponent :type Primitive%20Component%20Object%20Reference))
  (bind _transformhandleidentity (Variables|GizmoIdentity|GetTransformHandleIdentity))
  (bind _value (Utilities|Map|Find _transformhandleidentity CurrentComponent))
  (switch Utilities|FlowControl|Switch|SwitchonETransformMode (.transformmode _value)
    (:NewEnumerator0
      (Rendering|Material|SetMaterial CurrentComponent 0 "/Game/PointVRToolkit/Materials/TransformGizmo/MI_Hovered.MI_Hovered" :!label _label))
    (:NewEnumerator1
      (switch Utilities|FlowControl|Switch|SwitchonEConstraintAxis (.constraintaxis _value)
        (:NewEnumerator0
          (Rendering|Material|SetMaterial CurrentComponent 0 "/Game/PointVRToolkit/Materials/TransformGizmo/MI_Rotation_Hovered.MI_Rotation_Hovered" :!label _label_2))
        (:NewEnumerator1
          (goto _label_2))
        (:NewEnumerator2
          (goto _label_2))
        (:NewEnumerator8
          (Rendering|Material|SetMaterial CurrentComponent 0 "/Game/PointVRToolkit/Materials/TransformGizmo/MI_Trackball_Hovered.MI_Trackball_Hovered"))))
    (:NewEnumerator2
      (goto _label)))
  (return false))

(fn OnComponentUnhovered
  (params (Interactor :type BPC%20Toolkit%20Trace%20Interactor%20Object%20Reference) (TraceHit :type Hit%20Result%20Structure%20%28by%20ref%29) (PreviousComponent :type Primitive%20Component%20Object%20Reference))
  (bind _transformhandleidentity (Variables|GizmoIdentity|GetTransformHandleIdentity))
  (bind _value (Utilities|Map|Find _transformhandleidentity PreviousComponent))
  (switch Utilities|FlowControl|Switch|SwitchonETransformMode (.transformmode _value)
    (:NewEnumerator0
      (switch Utilities|FlowControl|Switch|SwitchonEConstraintAxis (.constraintaxis _value) :!label _label
        (:NewEnumerator0
          (Rendering|Material|SetMaterial PreviousComponent 0 "/Game/PointVRToolkit/Materials/TransformGizmo/MI_XAxis.MI_XAxis" :!label _label_2))
        (:NewEnumerator1
          (Rendering|Material|SetMaterial PreviousComponent 0 "/Game/PointVRToolkit/Materials/TransformGizmo/MI_YAxis.MI_YAxis" :!label _label_3))
        (:NewEnumerator2
          (Rendering|Material|SetMaterial PreviousComponent 0 "/Game/PointVRToolkit/Materials/TransformGizmo/MI_ZAxis.MI_ZAxis" :!label _label_4))
        (:NewEnumerator11
          (goto _label_2))
        (:NewEnumerator10
          (goto _label_3))
        (:NewEnumerator9
          (goto _label_4))
        (:NewEnumerator8
          (Rendering|Material|SetMaterial PreviousComponent 0 "/Game/PointVRToolkit/Materials/TransformGizmo/MI_XYZAxis.MI_XYZAxis"))))
    (:NewEnumerator1
      (switch Utilities|FlowControl|Switch|SwitchonEConstraintAxis (.constraintaxis _value)
        (:NewEnumerator0
          (Rendering|Material|SetMaterial PreviousComponent 0 "/Game/PointVRToolkit/Materials/TransformGizmo/MI_Rotation_XAxis.MI_Rotation_XAxis"))
        (:NewEnumerator1
          (Rendering|Material|SetMaterial PreviousComponent 0 "/Game/PointVRToolkit/Materials/TransformGizmo/MI_Rotation_YAxis.MI_Rotation_YAxis"))
        (:NewEnumerator2
          (Rendering|Material|SetMaterial PreviousComponent 0 "/Game/PointVRToolkit/Materials/TransformGizmo/MI_Rotation_ZAxis.MI_Rotation_ZAxis"))
        (:NewEnumerator8
          (Rendering|Material|SetMaterial PreviousComponent 0 "/Game/PointVRToolkit/Materials/TransformGizmo/MI_TrackBall.MI_TrackBall"))))
    (:NewEnumerator2
      (goto _label)))
  (return false))

(fn OnDragCanceled
  (params (Interactor :type BPC%20Toolkit%20Trace%20Interactor%20Object%20Reference) (TraceHit :type Hit%20Result%20Structure%20%28by%20ref%29))
  (Default|UnlockHovered Interactor)
  (return false))

(fn OnDragDetected
  (params (Interactor :type BPC%20Toolkit%20Trace%20Interactor%20Object%20Reference) (TraceHit :type Hit%20Result%20Structure%20%28by%20ref%29))
  (bind _hitcomponent (Collision|BreakHitResult TraceHit))
  (bind _returnvalue (Game|GetPlayerController 0))
  (bind _returnvalue_2 (Game|GetPlayerController 0))
  (bind _returnvalue_3 (Game|GetPlayerController 0))
  (bind _returnvalue_4 (Game|GetPlayerController 0))
  (bind _returnvalue_5 (Game|GetPlayerController 0))
  (bind _transformhandleidentity (Variables|GizmoIdentity|GetTransformHandleIdentity))
  (bind _trackballradius (Variables|GizmoSettings|GetTrackballRadius))
  (bind _trackballradius_2 (Variables|GizmoSettings|GetTrackballRadius))
  (bind _scalegizmoroot (Variables|Default|GetScaleGizmoRoot))
  (bind _rotationgizmoroot (Variables|Default|GetRotationGizmoRoot))
  (bind _value (Utilities|Map|Find _transformhandleidentity _hitcomponent))
  (bind (_locationx _locationy) (Game|Player|GetMousePosition _returnvalue_5))
  (bind (_locationx_2 _locationy_2) (Game|Player|GetMousePosition _returnvalue))
  (bind (_locationx_3 _locationy_3) (Game|Player|GetMousePosition _returnvalue_3))
  (bind _returnvalue_6 (Transformation|GetWorldLocation _rotationgizmoroot))
  (bind _returnvalue_7 (Transformation|GetWorldLocation _scalegizmoroot))
  (bind _returnvalue_8 (Math|Vector|GetForwardVector _scalegizmoroot))
  (bind _returnvalue_9 (Math|Vector|GetRightVector _scalegizmoroot))
  (bind _returnvalue_10 (Math|Vector|GetUpVector _scalegizmoroot))
  (Default|LockHovered Interactor)
  (Variables|GizmoIdentity|SetTransformMode (.transformmode _value))
  (Variables|GizmoIdentity|SetOrientType (.orienttype _value))
  (Variables|GizmoIdentity|SetConstraintAxis (.constraintaxis _value))
  (Variables|GizmoDrag|SetCameraTransform (Transformation|GetActorTransform (Game|GetPlayerCameraManager 0)))
  (switch Utilities|FlowControl|Switch|SwitchonETransformMode (Variables|GizmoIdentity|GetTransformMode)
    (:NewEnumerator1
      ;[1 1 0] Rotation
      (switch Utilities|FlowControl|Switch|SwitchonEOrientType (Variables|GizmoIdentity|GetOrientType)
        (:NewEnumerator0
          (switch Utilities|FlowControl|Switch|SwitchonEConstraintAxis (Variables|GizmoIdentity|GetConstraintAxis)
            (:NewEnumerator0
              (Variables|GizmoDrag|SetScreenDragConstraintAxis (Class|KismetMathLibrary|GetRotated2D (CallFunction|ConvertWorldLinetoScreenVector2D _returnvalue_2 _returnvalue_6 (* (Math|Vector|GetForwardVector _rotationgizmoroot) _trackballradius_2)) -9e+01)))
            (:NewEnumerator1
              (Variables|GizmoDrag|SetScreenDragConstraintAxis (Class|KismetMathLibrary|GetRotated2D (CallFunction|ConvertWorldLinetoScreenVector2D _returnvalue_2 _returnvalue_6 (* (Math|Vector|GetRightVector _rotationgizmoroot) _trackballradius_2)) -9e+01)))
            (:NewEnumerator2
              (Variables|GizmoDrag|SetScreenDragConstraintAxis (Class|KismetMathLibrary|GetRotated2D (CallFunction|ConvertWorldLinetoScreenVector2D _returnvalue_2 _returnvalue_6 (* (Math|Vector|GetUpVector _rotationgizmoroot) _trackballradius_2)) -9e+01))))
          (bind _output_get (Variables|GizmoDrag|SetCurrentScreenDragPosition (Math|Vector2D|MakeVector2D _locationx_3 _locationy_3)))
          (Variables|GizmoDrag|SetPreviousScreenDragPosition _output_get))
        (:NewEnumerator1
          (switch Utilities|FlowControl|Switch|SwitchonEConstraintAxis (Variables|GizmoIdentity|GetConstraintAxis)
            (:NewEnumerator8
              ;;[1 1 0] Trackball
              (bind _output_get_2 (Variables|GizmoDrag|SetArcballCenterScreenPosition (.ScreenPosition (Class|GameplayStatics|ProjectWorldtoScreen _returnvalue (Transformation|GetWorldLocation (Variables|Default|GetRotationGizmoRoot)) false))))
              (bind _output_get_3 (Variables|GizmoDrag|SetCurrentArcballVector (CallFunction|ConvertScreenLocationtoArcballVector (Math|Vector2D|MakeVector2D _locationx_2 _locationy_2) _output_get_2 (Variables|GizmoSettings|GetVirtualArcballRadius) (Variables|GizmoDrag|GetCameraTransform))))
              (Variables|GizmoDrag|SetPreviousArcballVector _output_get_3)))))
      (Variables|TransformTarget|SetTargetWorldRotation (Transformation|GetWorldRotation (Variables|TransformTarget|GetTransformTargetRoot)))
      (return true))
    (:NewEnumerator2
      ;[1 1 0] Scale
      (switch Utilities|FlowControl|Switch|SwitchonEOrientType (Variables|GizmoIdentity|GetOrientType)
        (:NewEnumerator0
          (switch Utilities|FlowControl|Switch|SwitchonEConstraintAxis (Variables|GizmoIdentity|GetConstraintAxis)
            (:NewEnumerator0
              (Variables|GizmoDrag|SetScreenDragConstraintAxis (CallFunction|ConvertWorldLinetoScreenVector2D _returnvalue_4 _returnvalue_7 (* (Math|Vector|GetForwardVector _scalegizmoroot) _trackballradius))))
            (:NewEnumerator1
              (Variables|GizmoDrag|SetScreenDragConstraintAxis (CallFunction|ConvertWorldLinetoScreenVector2D _returnvalue_4 _returnvalue_7 (* (Math|Vector|GetRightVector _scalegizmoroot) _trackballradius))))
            (:NewEnumerator2
              (Variables|GizmoDrag|SetScreenDragConstraintAxis (CallFunction|ConvertWorldLinetoScreenVector2D _returnvalue_4 _returnvalue_7 (* (Math|Vector|GetUpVector _scalegizmoroot) _trackballradius))))
            (:NewEnumerator11
              (Variables|GizmoDrag|SetScreenDragConstraintAxis (CallFunction|ConvertWorldLinetoScreenVector2D _returnvalue_4 _returnvalue_7 (* (+ _returnvalue_9 _returnvalue_10) _trackballradius))))
            (:NewEnumerator10
              (Variables|GizmoDrag|SetScreenDragConstraintAxis (CallFunction|ConvertWorldLinetoScreenVector2D _returnvalue_4 _returnvalue_7 (* (+ _returnvalue_8 _returnvalue_10) _trackballradius))))
            (:NewEnumerator9
              (Variables|GizmoDrag|SetScreenDragConstraintAxis (CallFunction|ConvertWorldLinetoScreenVector2D _returnvalue_4 _returnvalue_7 (* (+ _returnvalue_8 _returnvalue_9) _trackballradius))))
            (:NewEnumerator8
              (Variables|GizmoDrag|SetScreenDragConstraintAxis (CallFunction|ConvertWorldLinetoScreenVector2D _returnvalue_4 _returnvalue_7 (* (+ (Math|Vector|GetForwardVector _scalegizmoroot) (Math|Vector|GetRightVector _scalegizmoroot) (Math|Vector|GetUpVector _scalegizmoroot)) _trackballradius)))))
          (bind _output_get_4 (Variables|GizmoDrag|SetCurrentScreenDragPosition (Math|Vector2D|MakeVector2D _locationx _locationy)))
          (Variables|GizmoDrag|SetPreviousScreenDragPosition _output_get_4)
          (Variables|TransformTarget|SetTargetWorldScale3D (Transformation|GetWorldScale (Variables|TransformTarget|GetTransformTargetRoot)))
          (return true))))))

(fn OnDragMove
  (params (Interactor :type BPC%20Toolkit%20Trace%20Interactor%20Object%20Reference) (TraceHit :type Hit%20Result%20Structure%20%28by%20ref%29))
  (bind _returnvalue (Game|GetPlayerController 0))
  (bind _returnvalue_2 (Game|GetPlayerController 0))
  (bind _returnvalue_3 (Game|GetPlayerController 0))
  (bind _rotationgizmoroot (Variables|Default|GetRotationGizmoRoot))
  (bind (_locationx _locationy) (Game|Player|GetMousePosition _returnvalue))
  (bind (_locationx_2 _locationy_2) (Game|Player|GetMousePosition _returnvalue_2))
  (bind (_locationx_3 _locationy_3) (Game|Player|GetMousePosition _returnvalue_3))
  (switch Utilities|FlowControl|Switch|SwitchonETransformMode (Variables|GizmoIdentity|GetTransformMode)
    (:NewEnumerator1
      ;[1 1 0] Rotation
      (switch Utilities|FlowControl|Switch|SwitchonEOrientType (Variables|GizmoIdentity|GetOrientType)
        (:NewEnumerator0
          ;;[1 1 0.01] LocalRotation
          (switch Utilities|FlowControl|Switch|SwitchonEConstraintAxis (Variables|GizmoIdentity|GetConstraintAxis)
            (:NewEnumerator0
              (Variables|GizmoDrag|SetCurrentScreenDragPosition (Math|Vector2D|MakeVector2D _locationx_2 _locationy_2))
              (Variables|TransformTarget|SetTargetWorldRotation (Math|Rotator|CombineRotators (Variables|TransformTarget|GetTargetWorldRotation) (Math|Vector|RotatorfromAxisandAngle (Math|Vector|GetForwardVector _rotationgizmoroot) (* (Math|Vector2D|DotProduct(2D) (- (Variables|GizmoDrag|GetCurrentScreenDragPosition) (Variables|GizmoDrag|GetPreviousScreenDragPosition)) (Variables|GizmoDrag|GetScreenDragConstraintAxis)) (Variables|GizmoSettings|GetRotationFactor))))))
            (:NewEnumerator1
              (Variables|GizmoDrag|SetCurrentScreenDragPosition (Math|Vector2D|MakeVector2D _locationx_2 _locationy_2))
              (Variables|TransformTarget|SetTargetWorldRotation (Math|Rotator|CombineRotators (Variables|TransformTarget|GetTargetWorldRotation) (Math|Vector|RotatorfromAxisandAngle (Math|Vector|GetRightVector _rotationgizmoroot) (* (Math|Vector2D|DotProduct(2D) (- (Variables|GizmoDrag|GetCurrentScreenDragPosition) (Variables|GizmoDrag|GetPreviousScreenDragPosition)) (Variables|GizmoDrag|GetScreenDragConstraintAxis)) (Variables|GizmoSettings|GetRotationFactor))))))
            (:NewEnumerator2
              (Variables|GizmoDrag|SetCurrentScreenDragPosition (Math|Vector2D|MakeVector2D _locationx_2 _locationy_2))
              (Variables|TransformTarget|SetTargetWorldRotation (Math|Rotator|CombineRotators (Variables|TransformTarget|GetTargetWorldRotation) (Math|Vector|RotatorfromAxisandAngle (Math|Vector|GetUpVector _rotationgizmoroot) (* (Math|Vector2D|DotProduct(2D) (- (Variables|GizmoDrag|GetCurrentScreenDragPosition) (Variables|GizmoDrag|GetPreviousScreenDragPosition)) (Variables|GizmoDrag|GetScreenDragConstraintAxis)) (Variables|GizmoSettings|GetRotationFactor)))))))
          (Transformation|SetWorldRotation (Variables|TransformTarget|GetTransformTargetRoot) (Variables|TransformTarget|GetTargetWorldRotation) false false)
          (Transformation|SetWorldRotation (Variables|Default|GetRotationGizmoRoot) (Variables|TransformTarget|GetTargetWorldRotation) false false)
          (Variables|GizmoDrag|SetPreviousScreenDragPosition (Variables|GizmoDrag|GetCurrentScreenDragPosition)))
        (:NewEnumerator1
          (switch Utilities|FlowControl|Switch|SwitchonEConstraintAxis (Variables|GizmoIdentity|GetConstraintAxis)
            (:NewEnumerator8
              ;;[1 1 0] Arcball(Trackball)轨迹球只有世界坐标系
              (Variables|GizmoDrag|SetCurrentArcballVector (CallFunction|ConvertScreenLocationtoArcballVector (Math|Vector2D|MakeVector2D _locationx _locationy) (Variables|GizmoDrag|GetArcballCenterScreenPosition) (Variables|GizmoSettings|GetVirtualArcballRadius) (Variables|GizmoDrag|GetCameraTransform)))
              (bind _output_get (Variables|TransformTarget|SetTargetWorldRotation (Math|Rotator|CombineRotators (Variables|TransformTarget|GetTargetWorldRotation) (CallFunction|CalculateArcballDeltaRotation (Variables|GizmoDrag|GetPreviousArcballVector) (Variables|GizmoDrag|GetCurrentArcballVector)))))
              (Transformation|SetWorldRotation (Variables|TransformTarget|GetTransformTargetRoot) _output_get false false)
              (Transformation|SetWorldRotation (Variables|Default|GetRotationGizmoRoot) (Variables|TransformTarget|GetTargetWorldRotation) false false)
              (Variables|GizmoDrag|SetPreviousArcballVector (Variables|GizmoDrag|GetCurrentArcballVector))))))
      (return false))
    (:NewEnumerator2
      ;[1 1 0] Scale只有本地坐标系
      (switch Utilities|FlowControl|Switch|SwitchonEOrientType (Variables|GizmoIdentity|GetOrientType)
        (:NewEnumerator0
          (switch Utilities|FlowControl|Switch|SwitchonEConstraintAxis (Variables|GizmoIdentity|GetConstraintAxis)
            (:NewEnumerator0
              (Variables|GizmoDrag|SetCurrentScreenDragPosition (Math|Vector2D|MakeVector2D _locationx_3 _locationy_3))
              (Variables|TransformTarget|SetTargetWorldScale3D (+ (Math|Vector|MakeVector (* (Math|Vector2D|DotProduct(2D) (- (Variables|GizmoDrag|GetCurrentScreenDragPosition) (Variables|GizmoDrag|GetPreviousScreenDragPosition)) (Variables|GizmoDrag|GetScreenDragConstraintAxis)) (Variables|GizmoSettings|GetScaleFactor)) 0.0 0.0) (Variables|TransformTarget|GetTargetWorldScale3D))))
            (:NewEnumerator1
              (Variables|GizmoDrag|SetCurrentScreenDragPosition (Math|Vector2D|MakeVector2D _locationx_3 _locationy_3))
              (Variables|TransformTarget|SetTargetWorldScale3D (+ (Math|Vector|MakeVector 0.0 (* (Math|Vector2D|DotProduct(2D) (- (Variables|GizmoDrag|GetCurrentScreenDragPosition) (Variables|GizmoDrag|GetPreviousScreenDragPosition)) (Variables|GizmoDrag|GetScreenDragConstraintAxis)) (Variables|GizmoSettings|GetScaleFactor)) 0.0) (Variables|TransformTarget|GetTargetWorldScale3D))))
            (:NewEnumerator2
              (Variables|GizmoDrag|SetCurrentScreenDragPosition (Math|Vector2D|MakeVector2D _locationx_3 _locationy_3))
              (Variables|TransformTarget|SetTargetWorldScale3D (+ (Math|Vector|MakeVector 0.0 0.0 (* (Math|Vector2D|DotProduct(2D) (- (Variables|GizmoDrag|GetCurrentScreenDragPosition) (Variables|GizmoDrag|GetPreviousScreenDragPosition)) (Variables|GizmoDrag|GetScreenDragConstraintAxis)) (Variables|GizmoSettings|GetScaleFactor))) (Variables|TransformTarget|GetTargetWorldScale3D))))
            (:NewEnumerator11
              (Variables|GizmoDrag|SetCurrentScreenDragPosition (Math|Vector2D|MakeVector2D _locationx_3 _locationy_3))
              (Variables|TransformTarget|SetTargetWorldScale3D (+ (Math|Vector|MakeVector 0.0 (* (Math|Vector2D|DotProduct(2D) (- (Variables|GizmoDrag|GetCurrentScreenDragPosition) (Variables|GizmoDrag|GetPreviousScreenDragPosition)) (Variables|GizmoDrag|GetScreenDragConstraintAxis)) (Variables|GizmoSettings|GetScaleFactor)) (* (Math|Vector2D|DotProduct(2D) (- (Variables|GizmoDrag|GetCurrentScreenDragPosition) (Variables|GizmoDrag|GetPreviousScreenDragPosition)) (Variables|GizmoDrag|GetScreenDragConstraintAxis)) (Variables|GizmoSettings|GetScaleFactor))) (Variables|TransformTarget|GetTargetWorldScale3D))))
            (:NewEnumerator10
              (Variables|GizmoDrag|SetCurrentScreenDragPosition (Math|Vector2D|MakeVector2D _locationx_3 _locationy_3))
              (Variables|TransformTarget|SetTargetWorldScale3D (+ (Math|Vector|MakeVector (* (Math|Vector2D|DotProduct(2D) (- (Variables|GizmoDrag|GetCurrentScreenDragPosition) (Variables|GizmoDrag|GetPreviousScreenDragPosition)) (Variables|GizmoDrag|GetScreenDragConstraintAxis)) (Variables|GizmoSettings|GetScaleFactor)) 0.0 (* (Math|Vector2D|DotProduct(2D) (- (Variables|GizmoDrag|GetCurrentScreenDragPosition) (Variables|GizmoDrag|GetPreviousScreenDragPosition)) (Variables|GizmoDrag|GetScreenDragConstraintAxis)) (Variables|GizmoSettings|GetScaleFactor))) (Variables|TransformTarget|GetTargetWorldScale3D))))
            (:NewEnumerator9
              (Variables|GizmoDrag|SetCurrentScreenDragPosition (Math|Vector2D|MakeVector2D _locationx_3 _locationy_3))
              (Variables|TransformTarget|SetTargetWorldScale3D (+ (Math|Vector|MakeVector (* (Math|Vector2D|DotProduct(2D) (- (Variables|GizmoDrag|GetCurrentScreenDragPosition) (Variables|GizmoDrag|GetPreviousScreenDragPosition)) (Variables|GizmoDrag|GetScreenDragConstraintAxis)) (Variables|GizmoSettings|GetScaleFactor)) (* (Math|Vector2D|DotProduct(2D) (- (Variables|GizmoDrag|GetCurrentScreenDragPosition) (Variables|GizmoDrag|GetPreviousScreenDragPosition)) (Variables|GizmoDrag|GetScreenDragConstraintAxis)) (Variables|GizmoSettings|GetScaleFactor)) 0.0) (Variables|TransformTarget|GetTargetWorldScale3D))))
            (:NewEnumerator8
              (Variables|GizmoDrag|SetCurrentScreenDragPosition (Math|Vector2D|MakeVector2D _locationx_3 _locationy_3))
              (Variables|TransformTarget|SetTargetWorldScale3D (+ (Math|Conversions|ToVector(Float) (* (Math|Vector2D|DotProduct(2D) (- (Variables|GizmoDrag|GetCurrentScreenDragPosition) (Variables|GizmoDrag|GetPreviousScreenDragPosition)) (Variables|GizmoDrag|GetScreenDragConstraintAxis)) (Variables|GizmoSettings|GetScaleFactor))) (Variables|TransformTarget|GetTargetWorldScale3D)))))
          (Transformation|SetWorldScale3D (Variables|TransformTarget|GetTransformTargetRoot) (Variables|TransformTarget|GetTargetWorldScale3D))
          (Variables|GizmoDrag|SetPreviousScreenDragPosition (Variables|GizmoDrag|GetCurrentScreenDragPosition))
          (return false))))))

(fn OnTraceEnter
  (params (Interactor :type BPC%20Toolkit%20Trace%20Interactor%20Object%20Reference) (TraceHit :type Hit%20Result%20Structure%20%28by%20ref%29))
  (return false))

(fn OnTraceLeave
  (params (Interactor :type BPC%20Toolkit%20Trace%20Interactor%20Object%20Reference) (TraceHit :type Hit%20Result%20Structure%20%28by%20ref%29))
  (return false))

(fn OnTraceMove
  (params (Interactor :type BPC%20Toolkit%20Trace%20Interactor%20Object%20Reference) (TraceHit :type Hit%20Result%20Structure%20%28by%20ref%29))
  (return false))