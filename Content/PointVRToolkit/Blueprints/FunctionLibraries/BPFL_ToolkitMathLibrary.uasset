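; Blueprint function library of math helpers for screen-to-world interaction and arcball-style rotation in the PointVR toolkit.
; Arcball helpers map a screen point to a camera-oriented virtual-sphere vector, flattened outside the radius, and turn two vectors into a cross-axis, arccos-angle rotation.
; Planar variants return signed or absolute-heading angles around a chosen X, Y or Z axis.
; Other helpers project world lines to screen directions and intersect deprojected screen rays with world planes.
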(fn CalculateArcballAngleAroundAxis2D
  (params (Axis :type EOrientAxis%20Enum :default "NewEnumerator0") (A :type Vector) (B :type Vector))
  (bind (_x _y _z) (Math|Vector|BreakVector B))
  (bind (_x_2 _y_2 _z_2) (Math|Vector|BreakVector A))
  (bind _returnvalue (Math|Vector2D|Normalize2D (Math|Vector2D|MakeVector2D _x _z)))
  (bind _returnvalue_2 (Math|Vector2D|Normalize2D (Math|Vector2D|MakeVector2D _x_2 _z_2)))
  (bind _returnvalue_3 (Math|Vector2D|Normalize2D (Math|Vector2D|MakeVector2D _x_2 _y_2)))
  (bind _returnvalue_4 (Math|Vector2D|Normalize2D (Math|Vector2D|MakeVector2D _x _y)))
  (bind _returnvalue_5 (Math|Vector2D|Normalize2D (Math|Vector2D|MakeVector2D _y_2 _z_2)))
  (bind _returnvalue_6 (Math|Vector2D|Normalize2D (Math|Vector2D|MakeVector2D _y _z)))
  ;[1 1 0] 这里其实是轨迹球旋转的在平面上的特殊形式
  (switch Utilities|FlowControl|Switch|SwitchonEOrientAxis Axis
    (:NewEnumerator0
      (return (* (Class|KismetMathLibrary|DegAcos (Math|Vector2D|DotProduct(2D) _returnvalue_5 _returnvalue_6)) (Math|Float|Sign(Float) (Class|KismetMathLibrary|CrossProduct2D _returnvalue_5 _returnvalue_6)) -1.0)))
    (:NewEnumerator1
      (return (* (Class|KismetMathLibrary|DegAcos (Math|Vector2D|DotProduct(2D) _returnvalue_2 _returnvalue)) (Math|Float|Sign(Float) (Class|KismetMathLibrary|CrossProduct2D _returnvalue_2 _returnvalue)))))
    (:NewEnumerator2
      (return (* (Class|KismetMathLibrary|DegAcos (Math|Vector2D|DotProduct(2D) _returnvalue_3 _returnvalue_4)) (Math|Float|Sign(Float) (Class|KismetMathLibrary|CrossProduct2D _returnvalue_3 _returnvalue_4)))))))

(fn CalculateRotationAngleAroundAxis2D
  (params (Axis :type EOrientAxis%20Enum :default "NewEnumerator0") (Direction :type Vector))
  (bind (_x _y _z) (Math|Vector|BreakVector Direction))
  ;[1 1 0] 绕X轴旋转时，初始方向为Z轴；绕Y轴旋转时，初始方向为X轴；绕Z轴旋转时，初始方向为Y轴
  (switch Utilities|FlowControl|Switch|SwitchonEOrientAxis Axis
    (:NewEnumerator0
      (return (Class|KismetMathLibrary|DegAtan2 _y _z)))
    (:NewEnumerator1
      (return (Class|KismetMathLibrary|DegAtan2 _z _x)))
    (:NewEnumerator2
      (return (* (Class|KismetMathLibrary|DegAtan2 _x _y) -1.0)))))

(fn GetArcballRotationBetweenTwoVectors
  (params (A :type Vector) (B :type Vector))
  (bind _returnvalue (Math|Vector|Normalize A))
  (bind _returnvalue_2 (Math|Vector|Normalize B))
  (return (Math|Vector|RotatorfromAxisandAngle (Math|Vector|CrossProduct _returnvalue _returnvalue_2) (Class|KismetMathLibrary|DegAcos (Math|Vector|DotProduct _returnvalue _returnvalue_2)))))

(fn ConvertWorldLinetoScreenVector2D
  (params (Player :type Player%20Controller%20Object%20Reference) (Origin :type Vector) (Direction :type Vector) (Length :type Float%20%28single-precision%29))
  (return (Math|Vector2D|Normalize2D (- (.ScreenPosition (Class|GameplayStatics|ProjectWorldtoScreen Player (+ Origin (* Direction Length)) false)) (.ScreenPosition (Class|GameplayStatics|ProjectWorldtoScreen Player Origin false))))))

(fn ConvertScreenLocationtoArcballVector
  (params (ScreenLocation :type Vector%202D%20Structure) (ArcballCenter :type Vector%202D%20Structure) (ArcballRadius :type Float%20%28single-precision%29) (CameraTransform :type Transform%20%28by%20ref%29))
  (bind _returnvalue (- ScreenLocation ArcballCenter))
  (bind _returnvalue_2 (Math|Float|Square ArcballRadius))
  (bind _returnvalue_3 (Class|KismetMathLibrary|DistanceSquared2D ScreenLocation ArcballCenter))
  (bind _returnvalue_4 (* (.y _returnvalue) -1.0))
  (if (>= _returnvalue_2 _returnvalue_3)
    (return (Math|Vector|Normalize (Math|Transform|TransformDirection CameraTransform (Math|Vector|MakeVector (* (Math|Float|Sqrt (- _returnvalue_2 _returnvalue_3)) -1.0) (.x _returnvalue) _returnvalue_4))))
    (else
      (return (Math|Vector|Normalize (Math|Transform|TransformDirection CameraTransform (Math|Vector|MakeVector 0.0 (.x _returnvalue) _returnvalue_4)))))))

(fn ProjectScreenPointontoWorldPlane
  (params (Player :type Player%20Controller%20Object%20Reference) (ScreenPoint :type Vector%202D%20Structure) (LineLength :type Float%20%28single-precision%29) (WorldPlane :type Plane%20Structure%20%28by%20ref%29))
  (bind (_worldposition _worlddirection) (Class|GameplayStatics|DeprojectScreentoWorld Player ScreenPoint))
  (bind _returnvalue (* _worlddirection LineLength))
  (bind _returnvalue_2 (+ _worldposition _returnvalue))
  (bind (_t _intersection _returnvalue_3) (Class|KismetMathLibrary|LinePlaneIntersection _worldposition _returnvalue_2 WorldPlane))
  (return _intersection _returnvalue_3))