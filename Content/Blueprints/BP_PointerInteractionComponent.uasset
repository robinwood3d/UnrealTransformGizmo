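; Pointer component that lets the player hover, press and drag interactable actors via line traces.
; Each active tick it traces from viewport center, mouse cursor or its forward vector, tracking the pointed actor and component.
; It sends enter, move, leave, press and release events as interface messages.
; An accepted press starts a drag, pausing tracing and sending drag messages to that actor until release.
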(event Custom|EnableInteraction
  (Components|Activation|SetActive true false))

(event Custom|DisableInteraction
  (Components|Activation|SetActive false false)
  (Class|BPIPointerInteractable|OnPointerRelease(Message) (Variables|Interaction|GetPointedActor) self)
  (Class|BPIPointerInteractable|OnPointerLeave(Message) (Variables|Interaction|GetPointedActor) self)
  (Variables|Interaction|SetPointedActor 0)
  (Variables|Default|SetLastTraceHit ""))

(event Custom|PressPointer
  (bind _boutresultedindrag (Class|BPIPointerInteractable|OnPointerPress(Message) (Variables|Interaction|GetPointedActor) self))
  (Variables|Default|SetbIsDragging _boutresultedindrag))

(event Custom|ReleasePointer
  (Class|BPIPointerInteractable|OnPointerRelease(Message) (Variables|Interaction|GetPointedActor) self)
  (Variables|Default|SetbIsDragging false))

(event EventBeginPlay
  (CallFunction|EnableInteraction))

(event EventTick
  (params (DeltaSeconds :type Float%20%28single-precision%29))
  (if (Components|Activation|IsActive)
    (if (not (Variables|Default|GetbIsDragging))
      (CallFunction|UpdatePointerMove)
      (else
        (Class|BPIPointerInteractable|OnPointerDrag(Message) (Variables|Interaction|GetPointedActor) self)))))

(fn UpdatePointerMove
  (bind _returnvalue (Transformation|GetWorldLocation))
  (bind _returnvalue_2 (Game|GetPlayerController 0))
  (bind _returnvalue_3 (Game|GetPlayerController 0))
  (bind (_sizex _sizey) (HUD|GetViewportSize _returnvalue_3))
  (bind (_worldlocation _worlddirection) (Game|Player|ConvertMouseLocationToWorldSpace _returnvalue_2))
  (bind _returnvalue_4 (* _sizex 0.5))
  (bind _returnvalue_5 (* _sizey 0.5))
  (bind (_worldposition _worlddirection_2) (Class|GameplayStatics|DeprojectScreentoWorld _returnvalue_3 (Math|Vector2D|MakeVector2D _returnvalue_4 _returnvalue_5)))
  (switch Utilities|FlowControl|Switch|SwitchonEInteractionSource (Variables|Default|GetInteractionSource)
    (:NewEnumerator0
      (LocalVariables|SetTraceStart _worldposition)
      (LocalVariables|SetTraceEnd (+ _worldposition (* _worlddirection_2 (Variables|Default|GetInteractionDistance)))))
    (:NewEnumerator2
      (LocalVariables|SetTraceStart _returnvalue)
      (LocalVariables|SetTraceEnd (+ _returnvalue (* (Math|Vector|GetForwardVector) (Variables|Default|GetInteractionDistance)))))
    (:NewEnumerator1
      (LocalVariables|SetTraceStart _worldlocation)
      (LocalVariables|SetTraceEnd (+ _worldlocation (* _worlddirection (Variables|Default|GetInteractionDistance))))))
  (bind _outhit (Collision|LineTraceByChannel (LocalVariables|GetTraceStart) (LocalVariables|GetTraceEnd) (Variables|Default|GetTraceChannel) true 0 "None"))
  (bind _output_get (Variables|Default|SetLastTraceHit _outhit))
  (LocalVariables|SetHitActor (.HitActor (Collision|BreakHitResult _output_get)))
  (LocalVariables|SetHitComponent (.HitComponent (Collision|BreakHitResult _output_get)))
  (if (== (LocalVariables|GetHitActor) (Variables|Interaction|GetPointedActor))
    (Class|BPIPointerInteractable|OnPointerMove(Message) (Variables|Interaction|GetPointedActor) self)
    (if (not (== (LocalVariables|GetHitComponent) (Variables|Interaction|GetPointedComponent)))
      (Class|BPIPointerInteractable|OnPointerLeaveComponent(Message) (Variables|Interaction|GetPointedActor) self (Variables|Interaction|GetPointedComponent))
      (Class|BPIPointerInteractable|OnPointerEnterComponent(Message) (Variables|Interaction|GetPointedActor) self (LocalVariables|GetHitComponent))
      (Variables|Interaction|SetPointedComponent (LocalVariables|GetHitComponent)))
    (else
      (Class|BPIPointerInteractable|OnPointerLeaveComponent(Message) (Variables|Interaction|GetPointedActor) self (Variables|Interaction|GetPointedComponent))
      (Class|BPIPointerInteractable|OnPointerLeave(Message) (Variables|Interaction|GetPointedActor) self)
      (bind _returnvalue_6 (Class|BPIPointerInteractable|IsInteractable(Message) (LocalVariables|GetHitActor) self))
      (if _returnvalue_6
        (Class|BPIPointerInteractable|OnPointerEnter(Message) (LocalVariables|GetHitActor) self)
        (Variables|Interaction|SetPointedActor (LocalVariables|GetHitActor))
        (Class|BPIPointerInteractable|OnPointerEnterComponent(Message) (Variables|Interaction|GetPointedActor) self (LocalVariables|GetHitComponent))
        (Variables|Interaction|SetPointedComponent (LocalVariables|GetHitComponent))
        (else
          (Variables|Interaction|SetPointedActor 0)
          (Variables|Interaction|SetPointedComponent 0))))))

(fn GetLastTraceHit
  (return (Variables|Default|GetLastTraceHit)))

(fn GetObjectUnderPointer
  (return (Variables|Interaction|GetPointedActor)))