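; Orbit camera pawn with mouse navigation: right-drag orbits, middle-drag pans, the wheel dollies, and left-click drives PointerInteraction when not navigating.
; Tick samples mouse input unless the pointer is dragging, then feeds interpolation-smoothed orbit, pan and dolly.
; Pan and dolly scale with camera distance; dolly is clamped and pauses during IsZoomingOnSelected.
; Navigation input enables Tick, which switches itself off once IsNavigating reports all motion has settled.
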(event Custom|UpdateMouseInput
  (bind _returnvalue (Game|GetPlayerController 0))
  (bind (_deltax _deltay) (Class|PlayerController|GetInputMouseDelta _returnvalue))
  ;[1 1 0] 鼠标轴值的输入
  (if (not (Variables|/Game/Blueprints/BP_PointerInteractionComponent.BP_PointerInteractionComponent_C|GetbIsDragging (Variables|Default|GetPointerInteraction)))
    (Variables|CameraNavigation|SetDeltaMouseInput (Math|Vector2D|MakeVector2D _deltax _deltay))
    (Variables|CameraNavigation|SetMouseWheelInput (Class|Actor|GetInputAxisKeyValue))))

(event Custom|CameraOrbit
  (params (DeltaMouseInput :type Vector%202D%20Structure) (DeltaTime :type Float%20%28single-precision%29%20%28by%20ref%29))
  ;[1 1 0] 摄像机围绕旋转
  (Utilities|FlowControl|Sequence
    (:then_0
      (Variables|CameraNavigation|SetSmoothedOrbitVector (Class|KismetMathLibrary|Vector2DInterpto (Variables|CameraNavigation|GetSmoothedOrbitVector) (select (Variables|CameraNavigation|GetbIsOrbiting) DeltaMouseInput "") DeltaTime 2e+01)))
    (:then_1
      (Pawn|Input|AddControllerYawInput (.x (* (* (Variables|CameraNavigation|GetSmoothedOrbitVector) "(X=1.000000,Y=-1.000000)") (Variables|CameraNavigation|GetCameraRotationSpeed))))
      (Pawn|Input|AddControllerPitchInput (.y (* (* (Variables|CameraNavigation|GetSmoothedOrbitVector) "(X=1.000000,Y=-1.000000)") (Variables|CameraNavigation|GetCameraRotationSpeed)))))))

(event Custom|CameraPan
  (params (DeltaMouseInput :type Vector%202D%20Structure) (DeltaTime :type Float%20%28single-precision%29%20%28by%20ref%29))
  (bind (_x _y) (Math|Vector2D|BreakVector2D DeltaMouseInput))
  (bind _opcamera (Variables|Default|GetOPCamera))
  ;[1 1 0] 摄像机平移
  (Utilities|FlowControl|Sequence
    (:then_0
      (Variables|CameraNavigation|SetSmoothedPanDirection (Math|Interpolation|VInterpTo (Variables|CameraNavigation|GetSmoothedPanDirection) (Math|Vector|SelectVector (* (Math|Transform|TransformDirection (Transformation|GetWorldTransform _opcamera) (Math|Vector|MakeVector 0.0 _x _y)) (* (.x (Variables|/Script/Engine.SceneComponent|GetRelativeLocation _opcamera)) (Variables|CameraNavigation|GetCameraPanSpeed))) "0, 0, 0" (Variables|CameraNavigation|GetbIsPanning)) DeltaTime 2e+01)))
    (:then_1
      (Transformation|AddActorWorldOffset (Variables|CameraNavigation|GetSmoothedPanDirection)))))

(event Custom|CameraDolly
  (params (DeltaTime :type Float%20%28single-precision%29%20%28by%20ref%29))
  ;[1 1 0] 摄像机拉近拉远
  (if (not (Variables|CameraNavigation|GetbIsZoomingOnSelected))
    (Utilities|FlowControl|Sequence
      (:then_0
        (Variables|CameraNavigation|SetSmoothedDolly (Math|Interpolation|FInterpTo (Variables|CameraNavigation|GetSmoothedDolly) (Variables|CameraNavigation|GetMouseWheelInput) DeltaTime 1e+01)))
      (:then_1
        (bind _output_get (Variables|CameraNavigation|SetCameraXDistance (Math|Float|Clamp(Float) (- (Variables|CameraNavigation|GetCameraXDistance) (* (Variables|CameraNavigation|GetCameraXDistance) (Variables|CameraNavigation|GetSmoothedDolly) (Variables|CameraNavigation|GetCameraDollySpeed))) (Variables|CameraNavigation|GetCameraXMinDistance) (Variables|CameraNavigation|GetCameraXMaxDistance))))
        (Transformation|SetRelativeLocation (Variables|Default|GetOPCamera) (Math|Vector|MakeVector (* _output_get -1.0) 0.0 0.0) false false)))))

(event EventBeginPlay
  (Variables|/Script/Engine.PlayerController|SetbShowMouseCursor (Game|GetPlayerController 0) true)
  (Actor|Tick|SetActorTickEnabled false)
  (Variables|CameraNavigation|SetCameraXDistance (* (.x (Variables|/Script/Engine.SceneComponent|GetRelativeLocation (Variables|Default|GetOPCamera))) -1.0)))

(event EventTick
  (params (DeltaSeconds :type Float%20%28single-precision%29))
  (bind _deltamouseinput (Variables|CameraNavigation|GetDeltaMouseInput))
  (Utilities|FlowControl|Sequence
    (:then_0
      (CallFunction|UpdateMouseInput)
      (CallFunction|CameraOrbit _deltamouseinput DeltaSeconds)
      (CallFunction|CameraPan _deltamouseinput DeltaSeconds)
      (CallFunction|CameraDolly DeltaSeconds))
    (:then_1
      ;[1 1 0] 这个是遗留的优化方案，在不进行鼠标操作的时候关闭Tick更新
      (if (not (CallFunction|IsNavigating))
        (Actor|Tick|SetActorTickEnabled false)))))

(event Input|MouseEvents|MiddleMouseButton
  (params (Key :type Key%20Structure :default "None"))
  (:Pressed
    (Actor|Tick|SetActorTickEnabled true)
    (Variables|CameraNavigation|SetbIsPanning true))
  (:Released
    (Variables|CameraNavigation|SetbIsPanning false)))

(event Input|MouseEvents|RightMouseButton
  (params (Key :type Key%20Structure :default "None"))
  (:Pressed
    (Actor|Tick|SetActorTickEnabled true)
    (Variables|CameraNavigation|SetbIsOrbiting true))
  (:Released
    (Variables|CameraNavigation|SetbIsOrbiting false)))

(event Input|MouseEvents|MouseWheelDown
  (params (Key :type Key%20Structure :default "None"))
  (:Pressed
    (Actor|Tick|SetActorTickEnabled true)
    (Variables|CameraNavigation|SetbIsDolly true))
  (:Released
    (Variables|CameraNavigation|SetbIsDolly false)))

(event Input|MouseEvents|MouseWheelUp
  (params (Key :type Key%20Structure :default "None"))
  (:Pressed
    (Actor|Tick|SetActorTickEnabled true)
    (Variables|CameraNavigation|SetbIsDolly true))
  (:Released
    (Variables|CameraNavigation|SetbIsDolly false)))

(event Input|MouseEvents|LeftMouseButton
  (params (Key :type Key%20Structure :default "None"))
  (bind _pointerinteraction (Variables|Default|GetPointerInteraction))
  (:Pressed
    (if (not (CallFunction|IsNavigating))
      (Default|PressPointer _pointerinteraction)))
  (:Released
    (Default|ReleasePointer _pointerinteraction)))

(fn ConstructionScript
  (|CallParentFunction))

(fn IsNavigating
  (return (Math|Boolean|ORBoolean (or (Variables|CameraNavigation|GetbIsOrbiting) (Math|Vector|NotEqual(Vector) :A (Variables|CameraNavigation|GetSmoothedOrbitVector))) (or (Variables|CameraNavigation|GetbIsPanning) (Math|Vector|NotEqual(Vector) (Variables|CameraNavigation|GetSmoothedPanDirection) "0, 0, 0" 0.0001)) (or (Variables|CameraNavigation|GetbIsDolly) (!= (Variables|CameraNavigation|GetSmoothedDolly) 0.0)))))