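; Blueprint function library of math helpers for a transform gizmo.
; Arcball functions map screen points onto a virtual sphere in camera space, clamped to the rim outside its radius, and derive the axis-angle rotation between two such vectors.
; Other helpers turn world lines into normalized screen directions, intersect deprojected screen rays with world planes, and snap vectors to a grid in an arbitrary transform's local space.
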(fn GetArcballRotationBetweenTwoVectors
  (params (A :type Vector) (B :type Vector))
  (bind _returnvalue (Math|Vector|Normalize A))
  (bind _returnvalue_2 (Math|Vector|Normalize B))
  (return (Math|Vector|RotatorfromAxisandAngle (Math|Vector|CrossProduct _returnvalue _returnvalue_2) (Class|KismetMathLibrary|DegAcos (Math|Vector|DotProduct _returnvalue _returnvalue_2)))))

(fn ConvertWorldLinetoScreenVector2D
  (params (Player :type Player%20Controller%20Object%20Reference) (Origin :type Vector) (Direction :type Vector) (Length :type Float%20%28single-precision%29))
  (return (Math|Vector2D|Normalize2D (- (.ScreenPosition (Class|GameplayStatics|ProjectWorldtoScreen Player (+ Origin (* Direction Length)) false)) (.ScreenPosition (Class|GameplayStatics|ProjectWorldtoScreen Player Origin false))))))

(fn ConvertScreenLocationtoArcballVector
  (params (ScreenLocation :type Vector%202D%20Structure) (ArcballCenter :type Vector%202D%20Structure) (ArcballRadius :type Float%20%28single-precision%29) (CameraTransform :type Transform%20%28by%20ref%29))
  (bind _returnvalue (- ScreenLocation ArcballCenter))
  (bind _returnvalue_2 (Math|Float|Square ArcballRadius))
  (bind _returnvalue_3 (Class|KismetMathLibrary|DistanceSquared2D ScreenLocation ArcballCenter))
  (bind _returnvalue_4 (* (.y _returnvalue) -1.0))
  (if (>= _returnvalue_2 _returnvalue_3)
    (return (Math|Vector|Normalize (Math|Transform|TransformDirection CameraTransform (Math|Vector|MakeVector (* (Math|Float|Sqrt (- _returnvalue_2 _returnvalue_3)) -1.0) (.x _returnvalue) _returnvalue_4))))
    (else
      (return (Math|Vector|Normalize (Math|Transform|TransformDirection CameraTransform (Math|Vector|MakeVector 0.0 (.x _returnvalue) _returnvalue_4)))))))

(fn ProjectScreenPointontoWorldPlane
  (params (Player :type Player%20Controller%20Object%20Reference) (ScreenPoint :type Vector%202D%20Structure) (LineLength :type Float%20%28single-precision%29) (WorldPlane :type Plane%20Structure%20%28by%20ref%29))
  (bind (_worldposition _worlddirection) (Class|GameplayStatics|DeprojectScreentoWorld Player ScreenPoint))
  (bind _returnvalue (* _worlddirection LineLength))
  (bind _returnvalue_2 (+ _worldposition _returnvalue))
  (bind (_t _intersection _returnvalue_3) (Class|KismetMathLibrary|LinePlaneIntersection _worldposition _returnvalue_2 WorldPlane))
  (return _intersection _returnvalue_3))

(fn VectorSnappedtoTransformedGrid
  (params (GridTransform :type Transform%20%28by%20ref%29) (InVector :type Vector) (GridSize :type Float%20%28single-precision%29))
  (return (Math|Transform|TransformLocation GridTransform (Class|KismetMathLibrary|VectorSnappedtoGrid (Math|Transform|InverseTransformLocation GridTransform InVector) GridSize))))